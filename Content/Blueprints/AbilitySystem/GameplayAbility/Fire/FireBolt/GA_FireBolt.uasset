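; Fire Bolt gameplay ability that launches a projectile toward the location under the mouse.
; A target data task stores the hit location in MouseTarget, while its immediate output plays the cast montage.
; The avatar updates its facing through CombatInterface, then the ability waits for the Event.Montage.FireBolt gameplay event.
; That event spawns the projectile at the stored target and ends the ability.
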(event `self.K2_ActivateAbility`
  (bind (_asynctaskproxy _datahandle) (`TargetDataUnderMouse.CreateTargetDataUnderMouse` (struct) null false false)
    (:`then`
      (`|PlayMontage` (`self.GetOwningComponentFromActorInfo`) "/Game/Blueprints/Anim/AM_Cast_FireBolt.AM_Cast_FireBolt"
        (:`then`
          (bind _ascombat_interface (cast `CombatInterface` (`self.GetAvatarActorFromActorInfo`)))
          (`CombatInterface.UpdateFacingTarget` _ascombat_interface (`self.MouseTarget`))
          (`AbilityTask_WaitGameplayEvent.WaitGameplayEvent` (struct :`TagName` "Event.Montage.FireBolt") null
            (:`EventReceived`
              (`self.SpawnProjectile` (`self.MouseTarget`))
              (`self.K2_EndAbility`))))))
    (:`ValidData`
      (set `self.MouseTarget` (`.Location` (`GameplayStatics.BreakHitResult` (`AbilitySystemBlueprintLibrary.GetHitResultFromTargetData` _datahandle)))))))